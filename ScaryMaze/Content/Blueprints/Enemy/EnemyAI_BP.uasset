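; Enemy AI controller that drives an EnemyCharacter_BP pawn in response to seeing the player.
; On possess it caches the enemy character and runs a behavior tree.
; AI perception updates write the CanSeePlayer blackboard key whenever the sensed actor is the main player character.
; Walk and Run events forward to the cached enemy.
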(event OnTargetPerceptionUpdated(AIPerception)
  (params (Actor :type Actor%20Object%20Reference) (Stimulus :type AI%20Stimulus%20Structure))
  (Utilities|Casting|CastToMyScaryMazeMainCharacter Actor)
  (AI|Components|Blackboard|SetValueasBool (AI|GetBlackboard 0) (Utilities|Name|MakeLiteralName "CanSeePlayer") (.bSuccessfullySensed (Utilities|Struct|BreakAIStimulus Stimulus))))

(event Custom|Walk
  (Default|Walk (Variables|Default|GetEnemy)))

(event Custom|Run
  (Default|Run (Variables|Default|GetEnemy)))

(event EventOnPossess
  (params (PossessedPawn :type Pawn%20Object%20Reference))
  (bind _asenemy_character_bp (Utilities|Casting|CastToEnemyCharacter_BP PossessedPawn))
  (Variables|Default|SetEnemy _asenemy_character_bp)
  (AI|RunBehaviorTree))

(fn ConstructionScript)