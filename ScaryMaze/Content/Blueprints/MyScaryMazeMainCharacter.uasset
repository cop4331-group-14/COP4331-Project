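; First-person player character for a maze game, handling melee attacks, damage and death, and the player's UI.
; Left click traces forward from head height for pawns and damages a Goblin or Heraklios when a random attack roll beats its random defense roll, destroying it on death.
; DealDamage updates health, destroying the player and showing a death screen when dead.
; BeginPlay adds the health bar, and M toggles the main menu.
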(event Custom|DealDamage
  (params (Damage :type Float%20%28single-precision%29))
  (Class|ScaryMazeBaseCharacter|CalculateHealth Damage)
  (if (Variables|Default|GetIsDead)
    (Actor|DestroyActor)
    (bind _returnvalue (UserInterface|CreateWidget "/Game/MainMenu/DeathScreen.DeathScreen_C"))
    (UserInterface|Viewport|AddtoViewport _returnvalue 0)
    (Variables|/Script/Engine.PlayerController|SetbShowMouseCursor (Game|GetPlayerController 0) true)))

(event EventBeginPlay
  (bind _returnvalue (UserInterface|CreateWidget "/Game/Blueprints/Health/HealthBar.HealthBar_C"))
  (UserInterface|Viewport|AddtoViewport _returnvalue 0))

(event Input|MouseEvents|LeftMouseButton
  (params (Key :type Key%20Structure))
  (bind _capsulecomponent (Variables|Default|GetCapsuleComponent))
  (bind _returnvalue (Transformation|GetWorldLocation _capsulecomponent))
  (:Pressed
    (bind (_outhit _returnvalue_2) (Collision|LineTraceForObjects (+ _returnvalue "0, 0,65.000000") (+ (+ _returnvalue "0, 0,65.000000") (* (Math|Vector|GetForwardVector (Transformation|GetWorldRotation (Variables|Default|GetFirstPersonCameraComponent))) 3.5e+02)) (Utilities|Array|MakeArray "ObjectTypeQuery3") false 0 "None"))
    (if _returnvalue_2
      (bind _asgoblin (Utilities|Casting|CastToGoblin (.HitActor (Collision|BreakHitResult _outhit)))
        (:then
          (bind _output_get (Variables|Default|Setrandom%20defense (Math|Random|RandomIntegerinRange 0 (Variables|/Script/ScaryMaze.EnemyCharacter|GetDefense _asgoblin))))
          (bind _output_get_2 (Variables|Default|Setrandom%20attack (Math|Random|RandomIntegerinRange 0 (Variables|Default|GetAttackPower))))
          (if (< (- _output_get _output_get_2) 0)
            (Class|EnemyCharacter|CalculateHealth _asgoblin (Math|Conversions|ToFloat(Integer) (- _output_get _output_get_2)))
            (if (Variables|/Script/ScaryMaze.EnemyCharacter|GetIsDead _asgoblin)
              (Actor|DestroyActor _asgoblin)
              (Development|PrintString "Enemy Killed!"))))
        (:CastFailed
          (bind _asheraklios (Utilities|Casting|CastToHeraklios (.HitActor (Collision|BreakHitResult _outhit))))
          (bind _output_get_3 (Variables|Default|Setrandom%20defense (Math|Random|RandomIntegerinRange 0 (Variables|/Script/ScaryMaze.EnemyCharacter|GetDefense _asheraklios))))
          (bind _output_get_4 (Variables|Default|Setrandom%20attack (Math|Random|RandomIntegerinRange 0 (Variables|Default|GetAttackPower))))
          (if (<= (- _output_get_3 _output_get_4) 0)
            (Class|EnemyCharacter|CalculateHealth _asheraklios (Math|Conversions|ToFloat(Integer) (- _output_get_3 _output_get_4)))
            (if (Variables|/Script/ScaryMaze.EnemyCharacter|GetIsDead _asheraklios)
              (Actor|DestroyActor _asheraklios)
              (Development|PrintString "Enemy Killed!"))))))))

(event Input|KeyboardEvents|M
  (params (Key :type Key%20Structure))
  (:Pressed
    (if (Variables|Default|GetMenuOnScreen)
      (Variables|Default|SetMenuOnScreen false)
      (Viewport|RemoveAllWidgets)
      (else
        (Variables|Default|SetMenuOnScreen true)
        (bind _returnvalue (UserInterface|CreateWidget "/Game/MainMenu/MainMenu.MainMenu_C"))
        (UserInterface|Viewport|AddtoViewport _returnvalue 0)
        (Variables|/Script/Engine.PlayerController|SetbShowMouseCursor (Game|GetPlayerController 0) true)))))

(fn ConstructionScript)